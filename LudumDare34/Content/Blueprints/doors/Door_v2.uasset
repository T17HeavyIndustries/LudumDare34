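; Automatic sliding door Blueprint that opens when something overlaps its trigger box.
; A timeline Driver slides two panels along local X, one flagged negative, and moves two rotators that spin by a configurable turn count.
; Ending overlap stops the timeline, then reverses it after a short delay.
; The construction script caches each part's starting location and applies configurable box size, position and timeline play rate.
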(event OnComponentEndOverlap(Box)
  (params (OtherActor :type Actor%20Object%20Reference) (OtherComp :type Primitive%20Component%20Object%20Reference) (OtherBodyIndex :type Integer))
  (bind _rotator (Variables|Default|Getrotator))
  (bind _rotator_2 (Variables|Default|Getrotator_2))
  (Utilities|FlowControl|Sequence
    (:then_0
      (bind _driver (Timeline|Timeline%20-%20Door_Driver Stop)
        (:Update
          (Variables|Timeline|SetDriver _driver)
          (Utilities|FlowControl|Sequence
            (:then_0
              (CallFunction|MoveMesh (Variables|Timeline|GetDriver) (Variables|Default|Getw_D_5x5_Am) false (Variables|DoorSetup|GetDoor_Start_1_loc)))
            (:then_1
              (CallFunction|MoveMesh (Variables|Timeline|GetDriver) (Variables|Default|Getw_D_5x5_Nm) true (Variables|DoorSetup|GetDoor_Start_2_loc)))
            (:then_2
              (CallFunction|MoveMesh (Variables|Timeline|GetDriver) _rotator false (Variables|DoorSetup|GetRotator_1_loc))
              (CallFunction|RotateMesh (Variables|Timeline|GetDriver) _rotator))
            (:then_3
              (CallFunction|MoveMesh (Variables|Timeline|GetDriver) _rotator_2 false (Variables|DoorSetup|GetRotator_2_loc))
              (CallFunction|RotateMesh (Variables|Timeline|GetDriver) _rotator_2))))))
    (:then_1
      (Utilities|FlowControl|Delay 0.5)
      (Timeline|Timeline%20-%20Door_Driver Reverse))))

(event OnComponentBeginOverlap(Box)
  (params (OtherActor :type Actor%20Object%20Reference) (OtherComp :type Primitive%20Component%20Object%20Reference) (OtherBodyIndex :type Integer) (bFromSweep :type Boolean) (SweepResult :type Hit%20Result%20Structure%20%28by%20ref%29))
  (bind _rotator (Variables|Default|Getrotator))
  (bind _rotator_2 (Variables|Default|Getrotator_2))
  (bind _driver (Timeline|Timeline%20-%20Door_Driver Play)
    (:Update
      (Variables|Timeline|SetDriver _driver)
      (Utilities|FlowControl|Sequence
        (:then_0
          (CallFunction|MoveMesh (Variables|Timeline|GetDriver) (Variables|Default|Getw_D_5x5_Am) false (Variables|DoorSetup|GetDoor_Start_1_loc)))
        (:then_1
          (CallFunction|MoveMesh (Variables|Timeline|GetDriver) (Variables|Default|Getw_D_5x5_Nm) true (Variables|DoorSetup|GetDoor_Start_2_loc)))
        (:then_2
          (CallFunction|MoveMesh (Variables|Timeline|GetDriver) _rotator false (Variables|DoorSetup|GetRotator_1_loc))
          (CallFunction|RotateMesh (Variables|Timeline|GetDriver) _rotator))
        (:then_3
          (CallFunction|MoveMesh (Variables|Timeline|GetDriver) _rotator_2 false (Variables|DoorSetup|GetRotator_2_loc))
          (CallFunction|RotateMesh (Variables|Timeline|GetDriver) _rotator_2))))))

(fn ConstructionScript
  (Utilities|FlowControl|Sequence
    (:then_0
      (|D1_set)
      (|D2_set)
      (|R1_set)
      (|R2_set))
    (:then_1
      (Components|Box|SetBoxExtent (Variables|Default|GetBox) (Math|Vector|MakeVector (Variables|BoxValues|GetBox_X_Extent) (Variables|BoxValues|GetBox_Y_Extent) (Variables|BoxValues|GetBox_Z_Extent)) true)
      (Transformation|SetRelativeLocation (Variables|Default|GetBox) (Math|Vector|MakeVector (Variables|BoxValues|GetBox_X) (Variables|BoxValues|GetBox_Y) (Variables|BoxValues|GetBox_Z)) false false)
      (Components|Timeline|SetPlayRate (Variables|Default|GetTimeline%20-%20Door_Driver) (Variables|Timeline|GetTimeline_Scale)))))

(fn MoveMesh
  (params (Driver :type Float%20%28single-precision%29) (Mesh :type Static%20Mesh%20Component%20Object%20Reference) (Negative? :type Boolean) (Start_Loc :type Vector))
  (bind (_x _y _z) (Math|Vector|BreakVector Start_Loc))
  (bind _negative (LocalVariables|Getnegative))
  (Utilities|FlowControl|Sequence
    (:then_0
      (if Negative?
        (Utilities|NegateInt _negative)))
    (:then_1
      (Transformation|SetRelativeLocation Mesh (Math|Vector|Lerp(Vector) Start_Loc (Math|Vector|MakeVector (+ (* _negative (Variables|DoorSetup|GetDoor_End_X)) _x) _y _z) Driver) false false))))

(fn RotateMesh
  (params (Driver :type Float%20%28single-precision%29) (Mesh :type Static%20Mesh%20Component%20Object%20Reference))
  (Transformation|SetRelativeRotation Mesh (Math|Rotator|MakeRotator 9e+01 (* Driver (* 3.6e+02 (Variables|Timeline|GetTurns))) 0.0) false false))