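; Automatic double sliding door that opens when something overlaps its trigger box and closes when the overlap ends.
; A timeline plays forward or in reverse, lerping two mesh panels from their start locations to mirrored X targets.
; Both targets derive from the first panel's start X plus an end offset, with Y and Z zeroed.
; The construction script applies the trigger box's extent and position from variables.
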(event OnComponentEndOverlap(Box)
  (params (OtherActor :type Actor%20Object%20Reference) (OtherComp :type Primitive%20Component%20Object%20Reference) (OtherBodyIndex :type Integer))
  (bind _door_end_x (Variables|DoorSetup|GetDoor_End_X))
  (bind _door_start_1 (Variables|DoorSetup|GetDoor_Start_1))
  (bind _returnvalue (+ _door_end_x (.x _door_start_1)))
  (bind _returnvalue_2 (Math|Vector|MakeVector _returnvalue 0.0 0.0))
  (bind _driver (Timeline|Timeline%20-%20Door_Driver Reverse)
    (:Update
      (Transformation|SetRelativeLocation (Variables|Default|Getw_D_5x5_Am) (Math|Vector|Lerp(Vector) (Variables|DoorSetup|GetDoor_Start_1) _returnvalue_2 _driver) false false)
      (Transformation|SetRelativeLocation (Variables|Default|Getw_D_5x5_Nm) (Math|Vector|Lerp(Vector) (Variables|DoorSetup|GetDoor_Start_2) (Math|Vector|NegateVector _returnvalue_2) _driver) false false))))

(event OnComponentBeginOverlap(Box)
  (params (OtherActor :type Actor%20Object%20Reference) (OtherComp :type Primitive%20Component%20Object%20Reference) (OtherBodyIndex :type Integer) (bFromSweep :type Boolean) (SweepResult :type Hit%20Result%20Structure%20%28by%20ref%29))
  (bind _door_end_x (Variables|DoorSetup|GetDoor_End_X))
  (bind _door_start_1 (Variables|DoorSetup|GetDoor_Start_1))
  (bind _returnvalue (+ _door_end_x (.x _door_start_1)))
  (bind _returnvalue_2 (Math|Vector|MakeVector _returnvalue 0.0 0.0))
  (bind _driver (Timeline|Timeline%20-%20Door_Driver Play)
    (:Update
      (Transformation|SetRelativeLocation (Variables|Default|Getw_D_5x5_Am) (Math|Vector|Lerp(Vector) (Variables|DoorSetup|GetDoor_Start_1) _returnvalue_2 _driver) false false)
      (Transformation|SetRelativeLocation (Variables|Default|Getw_D_5x5_Nm) (Math|Vector|Lerp(Vector) (Variables|DoorSetup|GetDoor_Start_2) (Math|Vector|NegateVector _returnvalue_2) _driver) false false))))

(fn ConstructionScript
  (Components|Box|SetBoxExtent (Variables|Default|GetBox) (Math|Vector|MakeVector (Variables|BoxValues|GetBox_X_Extent) (Variables|BoxValues|GetBox_Y_Extent) (Variables|BoxValues|GetBox_Z_Extent)) true)
  (Transformation|SetRelativeLocation (Variables|Default|GetBox) (Math|Vector|MakeVector (Variables|BoxValues|GetBox_X) (Variables|BoxValues|GetBox_Y) (Variables|BoxValues|GetBox_Z)) false false))