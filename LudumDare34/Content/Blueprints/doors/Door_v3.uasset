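; Sliding double door with four gears, opened by a trigger box overlap or by ActivateDoor.
; A timeline Driver value slides the two panels and their gears apart along local X while spinning the gears, via MoveMesh and RotateMesh.
; Leaving the box pauses, then reverses it; ActivateDoor runs a duplicate moveDoor timeline that reverses after Delay2.
; The construction script caches start locations, sizes the trigger and sets timeline speed.
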(event OnComponentEndOverlap(Box)
  (params (OtherActor :type Actor%20Object%20Reference) (OtherComp :type Primitive%20Component%20Object%20Reference) (OtherBodyIndex :type Integer))
  (bind _gear1 (Variables|Default|GetGear1))
  (bind _gear2 (Variables|Default|GetGear2))
  (bind _gear3 (Variables|Default|GetGear3))
  (bind _gear4 (Variables|Default|GetGear4))
  (Utilities|FlowControl|Sequence
    (:then_0
      (bind _driver (Timeline|Timeline%20-%20Door_Driver Stop)
        (:Update
          (Variables|Timeline|SetDriver _driver)
          (Utilities|FlowControl|Sequence
            (:then_0
              (CallFunction|MoveMesh (Variables|Timeline|GetDriver) (Variables|Default|GetdoorF) false (Variables|DoorSetup|GetDoor_Start_1_loc)))
            (:then_1
              (CallFunction|MoveMesh (Variables|Timeline|GetDriver) (Variables|Default|GetdoorM) true (Variables|DoorSetup|GetDoor_Start_2_loc)))
            (:then_2
              (CallFunction|MoveMesh (Variables|Timeline|GetDriver) _gear1 true (Variables|DoorSetup|GetRotator_1_loc))
              (CallFunction|RotateMesh (Variables|Timeline|GetDriver) _gear1 true false))
            (:then_3
              (CallFunction|MoveMesh (Variables|Timeline|GetDriver) _gear2 true (Variables|DoorSetup|GetRotator_2_loc))
              (CallFunction|RotateMesh (Variables|Timeline|GetDriver) _gear2 false true))
            (:then_4
              (CallFunction|MoveMesh (Variables|Timeline|GetDriver) _gear3 false (Variables|DoorSetup|GetRotator_3_loc))
              (CallFunction|RotateMesh (Variables|Timeline|GetDriver) _gear3 false false))
            (:then_5
              (CallFunction|MoveMesh (Variables|Timeline|GetDriver) _gear4 false (Variables|DoorSetup|GetRotator_4_loc))
              (CallFunction|RotateMesh (Variables|Timeline|GetDriver) _gear4 true true))))))
    (:then_1
      (Utilities|FlowControl|Delay 0.5)
      (Timeline|Timeline%20-%20Door_Driver Reverse))))

(event OnComponentBeginOverlap(Box)
  (params (OtherActor :type Actor%20Object%20Reference) (OtherComp :type Primitive%20Component%20Object%20Reference) (OtherBodyIndex :type Integer) (bFromSweep :type Boolean) (SweepResult :type Hit%20Result%20Structure%20%28by%20ref%29))
  (bind _gear1 (Variables|Default|GetGear1))
  (bind _gear2 (Variables|Default|GetGear2))
  (bind _gear3 (Variables|Default|GetGear3))
  (bind _gear4 (Variables|Default|GetGear4))
  (bind _driver (Timeline|Timeline%20-%20Door_Driver Play)
    (:Update
      (Variables|Timeline|SetDriver _driver)
      (Utilities|FlowControl|Sequence
        (:then_0
          (CallFunction|MoveMesh (Variables|Timeline|GetDriver) (Variables|Default|GetdoorF) false (Variables|DoorSetup|GetDoor_Start_1_loc)))
        (:then_1
          (CallFunction|MoveMesh (Variables|Timeline|GetDriver) (Variables|Default|GetdoorM) true (Variables|DoorSetup|GetDoor_Start_2_loc)))
        (:then_2
          (CallFunction|MoveMesh (Variables|Timeline|GetDriver) _gear1 true (Variables|DoorSetup|GetRotator_1_loc))
          (CallFunction|RotateMesh (Variables|Timeline|GetDriver) _gear1 true false))
        (:then_3
          (CallFunction|MoveMesh (Variables|Timeline|GetDriver) _gear2 true (Variables|DoorSetup|GetRotator_2_loc))
          (CallFunction|RotateMesh (Variables|Timeline|GetDriver) _gear2 false true))
        (:then_4
          (CallFunction|MoveMesh (Variables|Timeline|GetDriver) _gear3 false (Variables|DoorSetup|GetRotator_3_loc))
          (CallFunction|RotateMesh (Variables|Timeline|GetDriver) _gear3 false false))
        (:then_5
          (CallFunction|MoveMesh (Variables|Timeline|GetDriver) _gear4 false (Variables|DoorSetup|GetRotator_4_loc))
          (CallFunction|RotateMesh (Variables|Timeline|GetDriver) _gear4 true true))))))

(event Custom|Activate%20Door
  (Utilities|FlowControl|Sequence
    (:then_0
      (|movedoor :!label _label))
    (:then_1
      (Utilities|FlowControl|Delay (Variables|Timeline|Getdelay2))
      (goto _label Reverse))))

(fn ConstructionScript
  (Utilities|FlowControl|Sequence
    (:then_0
      (Variables|DoorSetup|SetDoor_Start_1_loc (Variables|/Script/Engine.SceneComponent|GetRelativeLocation (Variables|Default|GetdoorF)))
      (Variables|DoorSetup|SetDoor_Start_2_loc (Variables|/Script/Engine.SceneComponent|GetRelativeLocation (Variables|Default|GetdoorM)))
      (Variables|DoorSetup|SetRotator_1_loc (Variables|/Script/Engine.SceneComponent|GetRelativeLocation (Variables|Default|GetGear1)))
      (Variables|DoorSetup|SetRotator_2_loc (Variables|/Script/Engine.SceneComponent|GetRelativeLocation (Variables|Default|GetGear2)))
      (Variables|DoorSetup|SetRotator_3_loc (Variables|/Script/Engine.SceneComponent|GetRelativeLocation (Variables|Default|GetGear3)))
      (Variables|DoorSetup|SetRotator_4_loc (Variables|/Script/Engine.SceneComponent|GetRelativeLocation (Variables|Default|GetGear4))))
    (:then_1
      (Components|Box|SetBoxExtent (Variables|Default|GetBox) (Math|Vector|MakeVector (Variables|BoxValues|GetBox_X_Extent) (Variables|BoxValues|GetBox_Y_Extent) (Variables|BoxValues|GetBox_Z_Extent)) true)
      (Transformation|SetRelativeLocation (Variables|Default|GetBox) (Math|Vector|MakeVector (Variables|BoxValues|GetBox_X) (Variables|BoxValues|GetBox_Y) (Variables|BoxValues|GetBox_Z)) false false)
      (Components|Timeline|SetPlayRate (Variables|Default|GetTimeline%20-%20Door_Driver) (Variables|Timeline|GetTimeline_Scale)))))

(fn MoveMesh
  (params (Driver :type Float%20%28single-precision%29) (Mesh :type Static%20Mesh%20Component%20Object%20Reference) (Negative? :type Boolean) (Start_Loc :type Vector))
  (bind (_x _y _z) (Math|Vector|BreakVector Start_Loc))
  (bind _negative (LocalVariables|Getnegative))
  (Utilities|FlowControl|Sequence
    (:then_0
      (if Negative?
        (Utilities|NegateInt _negative)))
    (:then_1
      (Transformation|SetRelativeLocation Mesh (Math|Vector|Lerp(Vector) Start_Loc (Math|Vector|MakeVector (+ (* _negative (Variables|DoorSetup|GetDoor_End_X)) _x) _y _z) Driver) false false))))

(fn RotateMesh
  (params (Driver :type Float%20%28single-precision%29) (Mesh :type Static%20Mesh%20Component%20Object%20Reference) (Negative :type Boolean) (Flipped :type Boolean))
  (Transformation|SetRelativeRotation Mesh (Math|Rotator|MakeRotator 0.0 (* Driver (* (Math|Float|SelectFloat -3.6e+02 3.6e+02 Negative) (Variables|Timeline|GetTurns))) (Math|Float|SelectFloat 1.8e+02 0.0 Flipped)) false false))