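; A Canvas-based player HUD that draws a centered crosshair plus health and speed readouts without UMG.
; On each DrawHUD, it paints the crosshair texture mid-screen, health text at the bottom left and speed text at the top right.
; Setter functions update health, speed and the hide flag, which suppresses both readouts along with the crosshair.
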(event EventDrawHUD
  (params (SizeX :type Integer) (SizeY :type Integer))
  (if (not (Variables|Default|GethideCrosshair))
    (Canvas|DrawTexture "/Game/Textures/crosshair.crosshair" (Math|Conversions|ToFloat(Integer) (- (/ SizeX 2) 16)) (Math|Conversions|ToFloat(Integer) (- (/ SizeY 2) 16)) 32.0 32.0 0.0 0.0 1.0 1.0 "(R=1.000000,G=1.000000,B=1.000000,A=1.000000)")
    (HUD|DrawText (Utilities|String|ToString(Text) (Variables|Default|GetHealth)) "(R=0.000000,G=0.000000,B=0.000000,A=1.000000)" 5e+01 (Math|Conversions|ToFloat(Integer) (- SizeY 50)) 0 1.0 false)
    (HUD|DrawText (Utilities|String|ToString(Text) (Variables|Default|GetSpeed)) "(R=0.000000,G=0.000000,B=0.000000,A=1.000000)" (Math|Conversions|ToFloat(Integer) (- SizeX 50)) 5e+01 0 1.0 false)))

(fn ConstructionScript)

(fn SetHideCrossHair
  (params (val :type Boolean))
  (Variables|Default|SethideCrosshair val))

(fn SetHealth
  (params (val :type Text))
  (Variables|Default|SetHealth val))

(fn SetSpeed
  (params (val :type Text))
  (Variables|Default|SetSpeed val))