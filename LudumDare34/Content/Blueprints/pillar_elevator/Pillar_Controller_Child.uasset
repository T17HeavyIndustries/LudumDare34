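; Pillar elevator controller child Blueprint that overrides the unlock check for a pillar elevator driven by switches.
; CheckUnlock scans SwitchArray and treats the pillar as locked if any switch's Event flag is false.
; When every switch is on it activates the PillarElevator, otherwise it lowers the pillar.
; The construction script only calls the parent's.
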(event Custom|Check%20Unlock
  (bind _pillar_elevator (Variables|Default|GetPillar_Elevator))
  (Variables|Default|SetLocked false)
  (for _array_element (Variables|Default|GetSwitch_Array)
    (if (not (Variables|/Game/Blueprints/pads/Switch_Pad_Parent.Switch_Pad_Parent_C|Getevent _array_element))
      (Variables|Default|SetLocked true)))
  (if (Variables|Default|GetLocked)
    (Default|LowerPillar _pillar_elevator)
    (else
      (Default|ActivatePillar _pillar_elevator true))))

(fn ConstructionScript
  (|CallParentFunction))