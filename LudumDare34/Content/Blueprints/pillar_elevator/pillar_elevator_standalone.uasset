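; Standalone pillar elevator that, when unlocked, rises by a configurable height after a box overlap, then lowers itself automatically.
; A delay sequence gated by a busy flag drives the Raise and Lower graphs, which lerp the mesh's relative location through timelines.
; Play rate scales inversely with travel height, and box collision is disabled during the trip.
; Emissive materials on child meshes show ready, moving and locked or waiting states.
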(event OnComponentBeginOverlap(Box)
  (params (OtherActor :type Actor%20Object%20Reference) (OtherComp :type Primitive%20Component%20Object%20Reference) (OtherBodyIndex :type Integer) (bFromSweep :type Boolean) (SweepResult :type Hit%20Result%20Structure%20%28by%20ref%29))
  (if (Variables|Default|GetUnlocked)
    (Utilities|FlowControl|Delay 0.4)
    (if (Variables|Default|GetOut)
      (Variables|Default|SetOut false)
      (CallFunction|RaisePillar (Variables|Default|GetZmove))
      (Utilities|FlowControl|Delay 4.0)
      (CallFunction|LowerPillar)
      (Utilities|FlowControl|Delay 2.0)
      (CallFunction|ChangeMat "/Game/Materials/Emissive/Emissive_Purple.Emissive_Purple")
      (Utilities|FlowControl|Delay 1.0)
      (Variables|Default|SetOut true)
      (CallFunction|ChangeMat "/Game/Materials/Emissive/Emissive_Cyan.Emissive_Cyan"))))

(event OnComponentEndOverlap(Box)
  (params (OtherActor :type Actor%20Object%20Reference) (OtherComp :type Primitive%20Component%20Object%20Reference) (OtherBodyIndex :type Integer)))

(event Custom|Raise_Pillar
  (params (old_Z :type Float%20%28single-precision%29))
  (|Raise old_Z old_Z))

(event Custom|Change%20Mat
  (params (Material :type Material%20Object%20Reference))
  (|Mat_2 Material))

(event Custom|Lower%20Pillar
  (|Lower))

(fn ConstructionScript
  (bind _zmove (Variables|Default|GetZmove))
  (bind _output_get (Variables|Default|SetStart_Loc (Variables|/Script/Engine.SceneComponent|GetRelativeLocation (Variables|Default|GetStaticMesh))))
  (Variables|Default|SetEnd_Loc (Math|Vector|MakeVector (.x _output_get) (.y _output_get) _zmove))
  (Components|Timeline|SetPlayRate (Variables|Default|GetTimeline_1) (/ 2e+03 _zmove))
  (if (Variables|Default|GetUnlocked)
    (Variables|Default|SetUnlocked true)
    (CallFunction|ChangeMat "/Game/Materials/Emissive/Emissive_Cyan.Emissive_Cyan")
    (else
      (CallFunction|ChangeMat "/Game/Materials/Emissive/Emissive_Purple.Emissive_Purple"))))