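; Child variant of the pillar elevator that, when unlocked, runs a timed raise-and-lower cycle whenever its Box1 trigger is overlapped.
; The overlap disables Box1, calls the inherited raise and lower functions between delays scaled partly by timeline play rate, switches emissive colors, then re-arms.
; Construction sinks and teleports the inherited Box downward, sets the unlock state and tints unlocked pillars cyan.
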(event OnComponentBeginOverlap(Box1)
  (params (OtherActor :type Actor%20Object%20Reference) (OtherComp :type Primitive%20Component%20Object%20Reference) (OtherBodyIndex :type Integer) (bFromSweep :type Boolean) (SweepResult :type Hit%20Result%20Structure%20%28by%20ref%29))
  (Development|PrintString "Col")
  (Collision|SetCollisionEnabled (Variables|Default|GetBox1) "NoCollision")
  (if (Variables|Default|GetUnlocked)
    (Utilities|FlowControl|Delay 0.4)
    (if (Variables|Default|GetOut)
      (Variables|Default|SetOut false)
      (CallFunction|RaisePillar (Variables|Default|GetZmove))
      (Collision|SetCollisionEnabled (Variables|Default|GetBox) "NoCollision")
      (Utilities|FlowControl|Delay (Variables|Default|Getdelay))
      (Utilities|FlowControl|Delay 0.5)
      (CallFunction|ChangeMat "/Game/Materials/Emissive/Emissive_Purple.Emissive_Purple")
      (Utilities|FlowControl|Delay 4.0)
      (CallFunction|LowerPillar)
      (Collision|SetCollisionEnabled (Variables|Default|GetBox) "NoCollision")
      (Utilities|FlowControl|Delay 2.0)
      (CallFunction|ChangeMat "/Game/Materials/Emissive/Emissive_Purple.Emissive_Purple")
      (Utilities|FlowControl|Delay 1.0)
      (Variables|Default|SetOut true)
      (CallFunction|ChangeMat "/Game/Materials/Emissive/Emissive_Cyan.Emissive_Cyan")
      (Collision|SetCollisionEnabled (Variables|Default|GetBox1) "QueryOnly")
      (Development|PrintString "enabled"))))

(fn ConstructionScript
  (|CallParentFunction)
  (Collision|SetCollisionEnabled (Variables|Default|GetBox1) "QueryOnly")
  (Variables|Default|SetUnlocked (Variables|Default|GetUnlock))
  (Transformation|SetRelativeLocation (Variables|Default|GetBox) "0, 0,-700.000000" false true)
  (Variables|Default|Setdelay (/ 2.0 (Components|Animation|GetPlayRate (Variables|Default|GetTimeline_1))))
  (if (Variables|Default|GetUnlock)
    (CallFunction|ChangeMat "/Game/Materials/Emissive/Emissive_Cyan.Emissive_Cyan")))