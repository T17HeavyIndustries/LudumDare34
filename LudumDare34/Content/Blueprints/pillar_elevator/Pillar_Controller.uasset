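; Pillar controller that unlocks a PillarElevator once every switch in its SwitchArray has fired its Event, using lights to show progress.
; CheckUnlock scans the switches: if any is active the lights turn green, then purple after a short delay; if none is active they turn red.
; When none remains inactive, it sets the elevator's Unlocked flag and turns it cyan, with the lights following after a delay.
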(event Custom|Check%20Unlock
  (bind _pillar_elevator (Variables|Default|GetPillar_Elevator))
  (bind _light_array (Variables|Default|GetLight_Array))
  (Variables|Default|Set1Event false)
  (Variables|Default|SetLocked false)
  (for _array_element (Variables|Default|GetSwitch_Array)
    (if (Variables|/Game/Blueprints/pads/Switch_Pad_Parent.Switch_Pad_Parent_C|Getevent _array_element)
      (if (not (Variables|Default|Get1Event))
        (Variables|Default|Set1Event true)
        (for _array_element_2 _light_array
          (Default|ChangeMat _array_element_2 "/Game/Materials/Emissive/Emissive_Green.Emissive_Green"))
        (Utilities|FlowControl|Delay 0.5)
        (for _array_element_3 (Variables|Default|GetLight_Array)
          (Default|ChangeMat _array_element_3 "/Game/Materials/Emissive/Emissive_Purple.Emissive_Purple")))
      (else
        (Variables|Default|SetLocked true))))
  (if (Variables|Default|GetLocked)
    (if (not (Variables|Default|Get1Event))
      (for _array_element_4 _light_array
        (Default|ChangeMat _array_element_4 "/Game/Materials/Emissive/Emissive_Red.Emissive_Red")))
    (else
      (Variables|/Game/Blueprints/pillar_elevator/pillar_elevator.pillar_elevator_C|SetUnlocked _pillar_elevator true)
      (Default|ChangeMat _pillar_elevator "/Game/Materials/Emissive/Emissive_Cyan.Emissive_Cyan")
      (Utilities|FlowControl|Delay 0.5)
      (for _array_element_5 _light_array
        (Default|ChangeMat _array_element_5 "/Game/Materials/Emissive/Emissive_Cyan.Emissive_Cyan")))))

(fn ConstructionScript)