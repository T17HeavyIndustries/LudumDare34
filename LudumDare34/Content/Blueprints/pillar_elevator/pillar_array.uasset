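; Pillar array actor for the pillar elevator feature that raises or lowers a group of pillars together.
; ActivatePillar stores the passed pillar and its Zmove, then loops over every entry in PillarArray.
; On raise, each pillar receives the smaller of its own Zmove and the passed pillar's, capping it at that height; otherwise each is lowered.
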(event Custom|Activate%20Pillar
  (params (Raise :type Boolean) (NewParam :type Pillar%20Elevator%20Object%20Reference))
  (Variables|Default|Setpillar NewParam)
  (Variables|Default|SetZmoveM (Variables|/Game/Blueprints/pillar_elevator/pillar_elevator.pillar_elevator_C|GetZmove NewParam))
  (for _array_element (Variables|Default|Getpillar_array)
    (if Raise
      (Default|RaisePillar _array_element (Math|Float|SelectFloat (Variables|Default|GetZmoveM) (Variables|/Game/Blueprints/pillar_elevator/pillar_elevator.pillar_elevator_C|GetZmove _array_element) (> (Variables|/Game/Blueprints/pillar_elevator/pillar_elevator.pillar_elevator_C|GetZmove _array_element) (Variables|Default|GetZmoveM))))
      (else
        (Default|LowerPillar _array_element)))))

(event EventBeginPlay)

(event EventActorBeginOverlap
  (params (OtherActor :type Actor%20Object%20Reference)))

(event EventTick
  (params (DeltaSeconds :type Float%20%28single-precision%29)))

(fn ConstructionScript)