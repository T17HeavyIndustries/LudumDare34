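; Pillar elevator that moves its cube vertically on timelines, as part of a pillar array.
; Stepping into an unlocked, non-child pillar's box notifies PillarArray after a short delay; separate events raise it to a given height or lower it.
; Raise speed is scaled by target height, and the box collision is switched off during the rise.
; Emissive materials on the cube's child meshes show locked, unlocked, moving and child states.
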(event OnComponentEndOverlap(Box)
  (params (OtherActor :type Actor%20Object%20Reference) (OtherComp :type Primitive%20Component%20Object%20Reference) (OtherBodyIndex :type Integer)))

(event OnComponentBeginOverlap(Box)
  (params (OtherActor :type Actor%20Object%20Reference) (OtherComp :type Primitive%20Component%20Object%20Reference) (OtherBodyIndex :type Integer) (bFromSweep :type Boolean) (SweepResult :type Hit%20Result%20Structure%20%28by%20ref%29))
  (if (Variables|Default|GetUnlocked)
    (CallFunction|ActivatePillar true)))

(event Custom|Raise_Pillar
  (params (old_Z :type Float%20%28single-precision%29))
  (|Raise_2 old_Z old_Z))

(event Custom|Activate_Pillar
  (params (Raise :type Boolean))
  (|Activate_2 Raise))

(event Custom|Change%20Mat
  (params (Material :type Material%20Object%20Reference))
  (|Mat Material))

(event Custom|Lower%20Pillar
  (|Lower_2))

(fn ConstructionScript
  (bind _output_get (Variables|Default|SetStart_Loc (Variables|/Script/Engine.SceneComponent|GetRelativeLocation (Variables|Default|GetCube))))
  (Variables|Default|SetEnd_Loc _output_get)
  (Components|Timeline|SetPlayRate (Variables|Default|GetTimeline_1) (/ 2e+03 (Variables|Default|GetZmove)))
  (Utilities|FlowControl|Sequence
    (:then_0
      (if (Variables|Default|GetChild)
        (Variables|Default|SetUnlocked true)
        (CallFunction|ChangeMat "/Game/Materials/Emissive/Emissive_Purple.Emissive_Purple")
        (else
          (CallFunction|ChangeMat "/Game/Materials/Emissive/Emissive_Red.Emissive_Red"))))))