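; Horizontal pillar elevator that slides its Cube along local X, starting on BeginPlay if Unlocked or whenever Activate is called.
; After a start delay, a timeline drives the position lerp and replays after each pause while Unlocked.
; Emissive materials on the Cube's child meshes show state: red when locked, green when active, purple during pauses.
; The construction script sets the initial color from Unlocked.
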(event Custom|Change%20Mat
  (params (Material :type Material%20Object%20Reference))
  (|Mat_2 Material))

(event Custom|Activate
  (CallFunction|ChangeMat "/Game/Materials/Emissive/Emissive_Green.Emissive_Green")
  (Utilities|FlowControl|Delay (Variables|Default|Getstart%20delay))
  (bind _driver (Timeline|Timeline_0 Play)
    (:Update
      (Transformation|SetRelativeLocation (Variables|Default|GetCube) (Math|Vector|Lerp(Vector) "0, 0, 0" "700.000000, 0, 0" _driver) false false))
    (:Finished
      (if (Variables|Default|GetUnlocked)
        (|DelayAndMaterial)
        (Timeline|Timeline_0 PlayFromStart)))))

(event EventBeginPlay
  (if (Variables|Default|GetUnlocked)
    (CallFunction|Activate)))

(fn ConstructionScript
  (if (Variables|Default|GetUnlocked)
    (CallFunction|ChangeMat "/Game/Materials/Emissive/Emissive_Green.Emissive_Green")
    (else
      (CallFunction|ChangeMat "/Game/Materials/Emissive/Emissive_Red.Emissive_Red"))))