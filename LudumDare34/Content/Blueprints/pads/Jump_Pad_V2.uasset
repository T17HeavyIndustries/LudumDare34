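; Jump pad actor that launches the player character when it enters the pad's box trigger.
; On overlap it casts the other actor to PlayerCharacter and calls LaunchCharacter.
; The launch velocity combines the box's up and right vectors scaled by Zaccel and Xaccel, so rotating the box aims the jump, with variables controlling XY and Z velocity override.
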(event OnComponentBeginOverlap(Box)
  (params (OtherActor :type Actor%20Object%20Reference) (OtherComp :type Primitive%20Component%20Object%20Reference) (OtherBodyIndex :type Integer) (bFromSweep :type Boolean) (SweepResult :type Hit%20Result%20Structure%20%28by%20ref%29))
  (bind _box (Variables|Default|GetBox))
  (bind _asplayer_character (Utilities|Casting|CastToPlayerCharacter OtherActor))
  (Character|LaunchCharacter _asplayer_character (+ (* (Math|Vector|GetUpVector _box) (Variables|Default|GetZaccel)) (* (Math|Vector|GetRightVector _box) (Variables|Default|GetXaccel))) (Variables|Default|GetXYoverride) (Variables|Default|GetZoverride)))

(event EventBeginPlay)

(event Collision|EventActorBeginOverlap
  (params (OtherActor :type Actor%20Object%20Reference)))

(event EventTick
  (params (DeltaSeconds :type Float%20%28single-precision%29)))

(fn ConstructionScript)