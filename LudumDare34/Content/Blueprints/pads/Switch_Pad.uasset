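; Switch pad actor that lets the player press E within its box trigger to activate a pillar with Raise set to false.
; Box overlap enables player input, opens a gate and sets the HUDBluePrint prompt to "E"; leaving disables input and clears the prompt.
; Pressing E passes through the gate to call ActivatePillar on PillarArray, passing the first array element.
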(event OnComponentBeginOverlap(Box)
  (params (OtherActor :type Actor%20Object%20Reference) (OtherComp :type Primitive%20Component%20Object%20Reference) (OtherBodyIndex :type Integer) (bFromSweep :type Boolean) (SweepResult :type Hit%20Result%20Structure%20%28by%20ref%29))
  (bind _returnvalue (Game|GetPlayerController 0))
  (bind _pillar_array (Variables|Default|GetPillar_array))
  (Input|EnableInput _returnvalue)
  (bind _ashudblue_print (Utilities|Casting|CastToHUDBluePrint (HUD|GetHUD _returnvalue)))
  (Variables|/Game/Blueprints/Misc/HUDBluePrint.HUDBluePrint_C|SettoDisplay _ashudblue_print "E")
  (Utilities|FlowControl|Gate true) ; enters at Open
)

(event OnComponentEndOverlap(Box)
  (params (OtherActor :type Actor%20Object%20Reference) (OtherComp :type Primitive%20Component%20Object%20Reference) (OtherBodyIndex :type Integer))
  (bind _returnvalue (Game|GetPlayerController 0))
  (Input|DisableInput _returnvalue)
  (bind _ashudblue_print (Utilities|Casting|CastToHUDBluePrint (HUD|GetHUD _returnvalue)))
  (Variables|/Game/Blueprints/Misc/HUDBluePrint.HUDBluePrint_C|SettoDisplay _ashudblue_print ""))

(event EventBeginPlay)

(event Collision|EventActorBeginOverlap
  (params (OtherActor :type Actor%20Object%20Reference)))

(event EventTick
  (params (DeltaSeconds :type Float%20%28single-precision%29)))

(event Input|KeyboardEvents|E
  (params (Key :type Key%20Structure :default "AnyKey"))
  (bind _pillar_array (Variables|Default|GetPillar_array))
  (:Pressed
    (Utilities|FlowControl|Gate true
      (:Exit
        (Default|ActivatePillar _pillar_array false (Utilities|Array|Get(acopy) (Variables|/Game/Blueprints/pillar_elevator/pillar_array.pillar_array_C|Getpillar_array _pillar_array)))))))

(fn ConstructionScript)