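; Elevator pad that lifts the player character by launching it upward and suspending its gravity.
; Overlapping the Trigger zeroes the character's gravity scale and launches it with a configurable Z velocity and override flags.
; Leaving the elevator bounds box restores gravity on the cached character, without checking which actor left.
; The Construction Script sizes that box from bounds variables and raises it by its half-height.
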(event OnComponentBeginOverlap(Trigger)
  (params (OtherActor :type Actor%20Object%20Reference) (OtherComp :type Primitive%20Component%20Object%20Reference) (OtherBodyIndex :type Integer) (bFromSweep :type Boolean) (SweepResult :type Hit%20Result%20Structure%20%28by%20ref%29))
  (bind _asplayer_character (Utilities|Casting|CastToPlayerCharacter OtherActor))
  (Variables|/Script/Engine.CharacterMovementComponent|SetGravityScale (Variables|/Script/Engine.Character|GetCharacterMovement _asplayer_character) 0.0)
  (Character|LaunchCharacter _asplayer_character (Math|Vector|MakeVector 0.0 0.0 (Variables|LaunchSetup|GetZaccel)) (Variables|LaunchSetup|GetXYoverride) (Variables|LaunchSetup|GetZoverride)))

(event OnComponentEndOverlap(Elevator_Bounds)
  (params (OtherActor :type Actor%20Object%20Reference) (OtherComp :type Primitive%20Component%20Object%20Reference) (OtherBodyIndex :type Integer))
  (Variables|/Script/Engine.CharacterMovementComponent|SetGravityScale (Variables|/Script/Engine.Character|GetCharacterMovement (stale OnComponentBeginOverlap(Trigger) _asplayer_character)) 1.0))

(event EventBeginPlay)

(event Collision|EventActorBeginOverlap
  (params (OtherActor :type Actor%20Object%20Reference)))

(event EventTick
  (params (DeltaSeconds :type Float%20%28single-precision%29)))

(fn ConstructionScript
  (bind _bounds_z (Variables|BoundsSetup|GetBounds_Z))
  (bind _elevator_bounds (Variables|Default|GetElevator_Bounds))
  (bind _relativelocation (Variables|/Script/Engine.SceneComponent|GetRelativeLocation _elevator_bounds))
  (Components|Box|SetBoxExtent (Variables|Default|GetElevator_Bounds) (Math|Vector|MakeVector (Variables|BoundsSetup|GetBounds_X) (Variables|BoundsSetup|GetBounds_Y) _bounds_z) true)
  (Transformation|SetRelativeLocation _elevator_bounds (Math|Vector|MakeVector (.x _relativelocation) (.y _relativelocation) _bounds_z) false false))