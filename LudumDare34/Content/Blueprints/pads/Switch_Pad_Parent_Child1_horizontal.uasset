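; Horizontal child variant of a switch pad that triggers a set of linked actors when something overlaps its box.
; On overlap it turns cyan, then sets Unlocked to false and calls Activate on every element of the Horiz array.
; It then switches its material to purple or red based on Toggle.
; End overlap has no effect, and construction defers to the parent.
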(event OnComponentEndOverlap(Box)
  (params (OtherActor :type Actor%20Object%20Reference) (OtherComp :type Primitive%20Component%20Object%20Reference) (OtherBodyIndex :type Integer))
  (if (Variables|Default|GetToggle)
    _))

(event OnComponentBeginOverlap(Box)
  (params (OtherActor :type Actor%20Object%20Reference) (OtherComp :type Primitive%20Component%20Object%20Reference) (OtherBodyIndex :type Integer) (bFromSweep :type Boolean) (SweepResult :type Hit%20Result%20Structure%20%28by%20ref%29))
  (CallFunction|ChangeMat "/Game/Materials/Emissive/Emissive_Cyan.Emissive_Cyan")
  (for _array_element (Variables|Default|GetHoriz)
    (Variables|/Game/Blueprints/pillar_elevator/pillar_horizontal.pillar_horizontal_C|SetUnlocked _array_element false)
    (Default|Activate _array_element))
  (if (Variables|Default|GetToggle)
    (CallFunction|ChangeMat "/Game/Materials/Emissive/Emissive_Purple.Emissive_Purple")
    (else
      (CallFunction|ChangeMat "/Game/Materials/Emissive/Emissive_Red.Emissive_Red"))))

(fn ConstructionScript
  (|CallParentFunction))