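; Pressure switch pad variant, derived from a parent pad, that signals linked pillar elevators and unlocks horizontal array actors when its box is overlapped.
; Overlap begin and end set the Event flag and run controller macros on both pillar arrays, with end delayed one second.
; Each macro turns the pillar elevator cyan, then red after two seconds, and calls CheckUnlock.
; Horizontal actors activate only on begin; the pad uses purple emissive.
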(event OnComponentBeginOverlap(Box)
  (params (OtherActor :type Actor%20Object%20Reference) (OtherComp :type Primitive%20Component%20Object%20Reference) (OtherBodyIndex :type Integer) (bFromSweep :type Boolean) (SweepResult :type Hit%20Result%20Structure%20%28by%20ref%29))
  (Variables|Default|Setevent true)
  (for _array_element (Variables|Default|GetPillar_Controller self)
    (|Controllerindex _array_element _array_element))
  (for _array_element_2 (Variables|Default|GetPillar%20Child)
    (|Controllerindex_2 _array_element_2 _array_element_2))
  (for _array_element_3 (Variables|Default|GetHoriz%20Array)
    (Variables|/Game/Blueprints/pillar_elevator/pillar_horizontal.pillar_horizontal_C|SetUnlocked _array_element_3 true)
    (Default|Activate _array_element_3))
  (CallFunction|ChangeMat "/Game/Materials/Emissive/Emissive_Purple.Emissive_Purple"))

(event OnComponentEndOverlap(Box)
  (params (OtherActor :type Actor%20Object%20Reference) (OtherComp :type Primitive%20Component%20Object%20Reference) (OtherBodyIndex :type Integer))
  (Variables|Default|Setevent false)
  (Utilities|FlowControl|Delay 1.0)
  (for _array_element (Variables|Default|GetPillar_Controller self)
    (|Controllerindex_3 _array_element _array_element))
  (for _array_element_2 (Variables|Default|GetPillar%20Child)
    (|Controllerindex_2_2 _array_element_2 _array_element_2)))

(event Custom|Change%20Mat
  (params (Material :type Material%20Object%20Reference))
  (Rendering|Material|SetMaterial (Variables|Default|Getspawn_item_2x2x-1) 2 Material))

(fn ConstructionScript
  (|CallParentFunction)
  (CallFunction|ChangeMat "/Game/Materials/Emissive/Emissive_Purple.Emissive_Purple"))