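; CubeArray is an actor that stores the starting positions of a set of cubes and can move them back there.
; The construction script appends each cube's world location to CubeLocations.
; The ResetLocation event, when ShouldReset is set, teleports each cube in Cubes to its stored location by matching index, without sweeping.
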(event Custom|ResetLocation
  (if (Variables|Default|GetShouldReset)
    (for (_array_element _array_index) (Variables|Default|GetCubes)
      (Transformation|SetActorLocation _array_element (Utilities|Array|Get(acopy) (Variables|Default|GetCubeLocations) _array_index) false false))))

(event EventBeginPlay)

(event EventActorBeginOverlap
  (params (OtherActor :type Actor%20Object%20Reference)))

(event EventTick
  (params (DeltaSeconds :type Float%20%28single-precision%29)))

(fn ConstructionScript
  (for _array_element (Variables|Default|GetCubes)
    (Utilities|Array|Add (Variables|Default|GetCubeLocations) (Transformation|GetActorLocation _array_element))))