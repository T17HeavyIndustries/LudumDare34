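; A level manager actor that resets cube arrays and returns the player to the start.
; Pressing R moves the player character to the PlayerStart, waits 1.5 seconds, then calls ResetLocation on every entry in CubeArrays.
; A SetResetValue event lets callers set the ShouldReset flag on a specific array by level index.
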(event Custom|SetResetValue
  (params (Value :type Boolean) (LevelIndex :type Integer))
  (Variables|/Game/Blueprints/Misc/CubeArray.CubeArray_C|SetShouldReset (Utilities|Array|Get(acopy) (Variables|Default|GetCubeArrays) LevelIndex) Value))

(event EventBeginPlay
  (Input|EnableInput (Game|GetPlayerController 0)))

(event EventActorBeginOverlap
  (params (OtherActor :type Actor%20Object%20Reference)))

(event EventTick
  (params (DeltaSeconds :type Float%20%28single-precision%29)))

(event Input|KeyboardEvents|R
  (params (Key :type Key%20Structure :default "AnyKey"))
  (:Pressed
    (Transformation|SetActorLocation (Game|GetPlayerCharacter 0) (Transformation|GetActorLocation (Variables|Default|GetPlayerStart)) false false)
    (Utilities|FlowControl|Delay 1.5)
    (for _array_element (Variables|Default|GetCubeArrays)
      (Default|ResetLocation _array_element))))

(fn ConstructionScript)