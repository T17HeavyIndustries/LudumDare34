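; Pushable cube that the player pushes with E or pulls with Q, one scaled step at a time.
; Four trigger boxes enable movement, set the direction from their forward vector and show a HUD prompt.
; Offset line traces check for obstacles, then timelines lerp the cube to its target, moving the player too when pulling.
; A game mode flag lets only one block move at once.
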(event OnComponentBeginOverlap(Box1)
  (params (OtherActor :type Actor%20Object%20Reference) (OtherComp :type Primitive%20Component%20Object%20Reference) (OtherBodyIndex :type Integer) (bFromSweep :type Boolean) (SweepResult :type Hit%20Result%20Structure%20%28by%20ref%29))
  (Utilities|Casting|CastToLudumDare34Character OtherActor)
  (Variables|Default|SetcanMove true)
  (Variables|Default|Setforward (Math|Vector|GetForwardVector (Variables|Default|GetBox1)))
  (bind _ashudblue_print (Utilities|Casting|CastToHUDBluePrint (HUD|GetHUD (Game|GetPlayerController 0))))
  (Variables|/Game/Blueprints/Misc/HUDBluePrint.HUDBluePrint_C|SettoDisplay _ashudblue_print "E to push   Q to pull"))

(event OnComponentEndOverlap(Box1)
  (params (OtherActor :type Actor%20Object%20Reference) (OtherComp :type Primitive%20Component%20Object%20Reference) (OtherBodyIndex :type Integer))
  (Utilities|Casting|CastToLudumDare34Character OtherActor)
  (Variables|Default|SetcanMove false)
  (bind _ashudblue_print (Utilities|Casting|CastToHUDBluePrint (HUD|GetHUD (Game|GetPlayerController 0))))
  (Variables|/Game/Blueprints/Misc/HUDBluePrint.HUDBluePrint_C|SettoDisplay _ashudblue_print ""))

(event OnComponentBeginOverlap(Box2)
  (params (OtherActor :type Actor%20Object%20Reference) (OtherComp :type Primitive%20Component%20Object%20Reference) (OtherBodyIndex :type Integer) (bFromSweep :type Boolean) (SweepResult :type Hit%20Result%20Structure%20%28by%20ref%29))
  (Utilities|Casting|CastToLudumDare34Character OtherActor)
  (Variables|Default|SetcanMove true)
  (Variables|Default|Setforward (Math|Vector|GetForwardVector (Variables|Default|GetBox2)))
  (bind _ashudblue_print (Utilities|Casting|CastToHUDBluePrint (HUD|GetHUD (Game|GetPlayerController 0))))
  (Variables|/Game/Blueprints/Misc/HUDBluePrint.HUDBluePrint_C|SettoDisplay _ashudblue_print "E to push   Q to pull"))

(event OnComponentEndOverlap(Box2)
  (params (OtherActor :type Actor%20Object%20Reference) (OtherComp :type Primitive%20Component%20Object%20Reference) (OtherBodyIndex :type Integer))
  (Utilities|Casting|CastToLudumDare34Character OtherActor)
  (Variables|Default|SetcanMove false)
  (bind _ashudblue_print (Utilities|Casting|CastToHUDBluePrint (HUD|GetHUD (Game|GetPlayerController 0))))
  (Variables|/Game/Blueprints/Misc/HUDBluePrint.HUDBluePrint_C|SettoDisplay _ashudblue_print ""))

(event OnComponentBeginOverlap(Box3)
  (params (OtherActor :type Actor%20Object%20Reference) (OtherComp :type Primitive%20Component%20Object%20Reference) (OtherBodyIndex :type Integer) (bFromSweep :type Boolean) (SweepResult :type Hit%20Result%20Structure%20%28by%20ref%29))
  (Utilities|Casting|CastToLudumDare34Character OtherActor)
  (Variables|Default|SetcanMove true)
  (Variables|Default|Setforward (Math|Vector|GetForwardVector (Variables|Default|GetBox3)))
  (bind _ashudblue_print (Utilities|Casting|CastToHUDBluePrint (HUD|GetHUD (Game|GetPlayerController 0))))
  (Variables|/Game/Blueprints/Misc/HUDBluePrint.HUDBluePrint_C|SettoDisplay _ashudblue_print "E to push   Q to pull"))

(event OnComponentEndOverlap(Box3)
  (params (OtherActor :type Actor%20Object%20Reference) (OtherComp :type Primitive%20Component%20Object%20Reference) (OtherBodyIndex :type Integer))
  (Utilities|Casting|CastToLudumDare34Character OtherActor)
  (Variables|Default|SetcanMove false)
  (bind _ashudblue_print (Utilities|Casting|CastToHUDBluePrint (HUD|GetHUD (Game|GetPlayerController 0))))
  (Variables|/Game/Blueprints/Misc/HUDBluePrint.HUDBluePrint_C|SettoDisplay _ashudblue_print ""))

(event OnComponentBeginOverlap(Box)
  (params (OtherActor :type Actor%20Object%20Reference) (OtherComp :type Primitive%20Component%20Object%20Reference) (OtherBodyIndex :type Integer) (bFromSweep :type Boolean) (SweepResult :type Hit%20Result%20Structure%20%28by%20ref%29))
  (Utilities|Casting|CastToLudumDare34Character OtherActor)
  (Variables|Default|SetcanMove true)
  (Variables|Default|Setforward (Math|Vector|GetForwardVector (Variables|Default|GetBox)))
  (bind _ashudblue_print (Utilities|Casting|CastToHUDBluePrint (HUD|GetHUD (Game|GetPlayerController 0))))
  (Variables|/Game/Blueprints/Misc/HUDBluePrint.HUDBluePrint_C|SettoDisplay _ashudblue_print "E to push   Q to pull"))

(event OnComponentEndOverlap(Box)
  (params (OtherActor :type Actor%20Object%20Reference) (OtherComp :type Primitive%20Component%20Object%20Reference) (OtherBodyIndex :type Integer))
  (Utilities|Casting|CastToLudumDare34Character OtherActor)
  (Variables|Default|SetcanMove false)
  (bind _ashudblue_print (Utilities|Casting|CastToHUDBluePrint (HUD|GetHUD (Game|GetPlayerController 0))))
  (Variables|/Game/Blueprints/Misc/HUDBluePrint.HUDBluePrint_C|SettoDisplay _ashudblue_print ""))

(event EventBeginPlay
  (bind _forward (Variables|Default|Getforward))
  (bind _cube (Variables|Default|GetCube))
  (bind _returnvalue (Transformation|GetWorldScale _cube))
  (bind _returnvalue_2 (Transformation|GetWorldLocation _cube))
  (bind _x (Math|Vector|BreakVector _returnvalue))
  (Input|EnableInput (Game|GetPlayerController 0))
  (Utilities|FlowControl|Gate true) ; enters at Open
)

(event EventActorBeginOverlap
  (params (OtherActor :type Actor%20Object%20Reference)))

(event EventTick
  (params (DeltaSeconds :type Float%20%28single-precision%29)))

(event Input|KeyboardEvents|Q
  (params (Key :type Key%20Structure :default "AnyKey"))
  (bind _returnvalue (Game|GetPlayerCharacter 0))
  (bind _forward (Variables|Default|Getforward))
  (bind _forward_2 (Variables|Default|Getforward))
  (bind _cube (Variables|Default|GetCube))
  (bind _forward_3 (Variables|Default|Getforward))
  (bind _returnvalue_2 (Transformation|GetWorldScale _cube))
  (bind _returnvalue_3 (Transformation|GetWorldLocation _cube))
  (bind _returnvalue_4 (* _forward_3 -100))
  (bind _returnvalue_5 (VehicleSound|GetRootComponent _returnvalue))
  (bind _x (Math|Vector|BreakVector _returnvalue_2))
  (bind _returnvalue_6 (Transformation|GetWorldLocation _returnvalue_5))
  (bind _returnvalue_7 (* _returnvalue_4 _returnvalue_2))
  (bind _returnvalue_8 (* -25.0 _x))
  (bind _returnvalue_9 (* 25.0 _x))
  (:Pressed
    (Utilities|FlowControl|Gate false
      (:Exit
        (if (and (Variables|Default|GetcanMove) (not (Variables|Default|GetisMoving)))
          (bind _washit (CallFunction|TraceatHeight 5e+01 _returnvalue_3 _returnvalue_2 -2e+02 _forward _returnvalue_8))
          (if (not _washit)
            (bind _washit_2 (CallFunction|TraceatHeight 5e+01 _returnvalue_3 _returnvalue_2 -2e+02 _forward _returnvalue_9))
            (if (not _washit_2)
              (bind _washit_3 (CallFunction|TraceatHeight 1e+01 _returnvalue_3 _returnvalue_2 -1e+02 _forward_2 _returnvalue_8))
              (if (not _washit_3)
                (bind _washit_4 (CallFunction|TraceatHeight 1e+01 _returnvalue_3 _returnvalue_2 -1e+02 _forward_2 _returnvalue_9))
                (if (not _washit_4)
                  (bind _asgame_mode_blue_print (Utilities|Casting|CastToGameModeBluePrint (Game|GetGameMode)))
                  (if (not (Variables|/Game/Blueprints/Misc/GameModeBluePrint.GameModeBluePrint_C|GetstopTheFuckingBlocks _asgame_mode_blue_print))
                    (Variables|/Game/Blueprints/Misc/GameModeBluePrint.GameModeBluePrint_C|SetstopTheFuckingBlocks _asgame_mode_blue_print true)
                    (Variables|Default|SetisMoving true)
                    (bind _output_get (Variables|Default|SetendLocation (+ _returnvalue_3 _returnvalue_7)))
                    (Variables|Default|SetplayerEndLoc (+ _returnvalue_6 _returnvalue_7))
                    (bind _newtrack_0 (Timeline|Timeline_0 PlayFromStart)
                      (:Update
                        (Transformation|SetRelativeLocation (Variables|Default|GetCube) (Math|Vector|Lerp(Vector) _returnvalue_3 _output_get _newtrack_0) false false)
                        (Transformation|SetRelativeLocation (Variables|/Script/Engine.Character|GetCapsuleComponent _returnvalue) (Math|Vector|Lerp(Vector) _returnvalue_6 (Variables|Default|GetplayerEndLoc) _newtrack_0) false false))
                      (:Finished
                        (Variables|Default|SetisMoving false)
                        (Variables|/Game/Blueprints/Misc/GameModeBluePrint.GameModeBluePrint_C|SetstopTheFuckingBlocks _asgame_mode_blue_print false)))))))))))))

(event Input|KeyboardEvents|E
  (params (Key :type Key%20Structure :default "AnyKey"))
  (bind _forward (Variables|Default|Getforward))
  (bind _cube (Variables|Default|GetCube))
  (bind _returnvalue (Transformation|GetWorldScale _cube))
  (bind _returnvalue_2 (Transformation|GetWorldLocation _cube))
  (bind _x (Math|Vector|BreakVector _returnvalue))
  (:Pressed
    (Utilities|FlowControl|Gate true
      (:Exit
        (if (and (Variables|Default|GetcanMove) (not (Variables|Default|GetisMoving)))
          (bind _washit (CallFunction|TraceatHeight 1e+01 _returnvalue_2 _returnvalue 1e+02 _forward (* 25.0 _x)))
          (if (not _washit)
            (bind _washit_2 (CallFunction|TraceatHeight 1e+01 _returnvalue_2 _returnvalue 1e+02 _forward (* -25.0 _x)))
            (if (not _washit_2)
              (bind _asgame_mode_blue_print (Utilities|Casting|CastToGameModeBluePrint (Game|GetGameMode)))
              (if (not (Variables|/Game/Blueprints/Misc/GameModeBluePrint.GameModeBluePrint_C|GetstopTheFuckingBlocks _asgame_mode_blue_print))
                (Variables|/Game/Blueprints/Misc/GameModeBluePrint.GameModeBluePrint_C|SetstopTheFuckingBlocks _asgame_mode_blue_print true)
                (Variables|Default|SetisMoving true)
                (bind _output_get (Variables|Default|SetendLocation (+ _returnvalue_2 (* (* (Variables|Default|Getforward) 100) _returnvalue))))
                (bind _newtrack_0 (Timeline|Timeline_1 PlayFromStart)
                  (:Update
                    (Transformation|SetRelativeLocation (Variables|Default|GetCube) (Math|Vector|Lerp(Vector) _returnvalue_2 _output_get _newtrack_0) false false))
                  (:Finished
                    (Variables|Default|SetisMoving false)
                    (Variables|/Game/Blueprints/Misc/GameModeBluePrint.GameModeBluePrint_C|SetstopTheFuckingBlocks _asgame_mode_blue_print false)))))))))))

(fn ConstructionScript)

(fn GetRayVector
  (params (CenterVector :type Vector) (Scale :type Vector) (Height :type Float%20%28single-precision%29) (SideOffset :type Float%20%28single-precision%29) (Forward :type Vector))
  (bind (_x _y _z) (Math|Vector|BreakVector CenterVector))
  (bind _x_2 (Math|Vector|BreakVector Scale))
  (bind (_x_3 _y_2) (Math|Vector|BreakVector Forward))
  (bind _returnvalue (* 5e+01 _x_2))
  (bind _returnvalue_2 (- _z _returnvalue))
  (bind _returnvalue_3 (+ _returnvalue_2 Height))
  (Math|Float|CompareFloat (Math|Float|Absolute(Float) _x_3) (Math|Float|Absolute(Float) _y_2)
    (:>
      (return (Math|Vector|MakeVector _x (+ _y SideOffset) _returnvalue_3)))
    (:<
      (return (Math|Vector|MakeVector (+ _x SideOffset) _y _returnvalue_3)))))

(fn TraceatHeight
  (params (height :type Float%20%28single-precision%29) (center :type Vector) (scale :type Vector) (Distance :type Float%20%28single-precision%29) (Forward :type Vector) (sideOffset :type Float%20%28single-precision%29))
  (bind _return (CallFunction|GetRayVector center scale height sideOffset Forward))
  (bind _returnvalue (Collision|LineTraceForObjects _return (+ _return (* (* Forward scale) Distance)) (Utilities|Array|MakeArray "ObjectTypeQuery1" "ObjectTypeQuery2" "ObjectTypeQuery4") false 0 "Persistent"))
  (return _returnvalue))