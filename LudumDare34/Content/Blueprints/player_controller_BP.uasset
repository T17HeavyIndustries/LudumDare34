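; Player controller Blueprint that feeds the local player's status to a non-UMG HUD every frame.
; Tick pushes the character's horizontal speed and current health as text to PlayerHUDnonUMG while the player is alive.
; It also compares the dead state with the previous frame's cached value, hiding the crosshair on death and showing it again when alive.
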(event EventBeginPlay)

(event EventTick
  (params (DeltaSeconds :type Float%20%28single-precision%29))
  (CallFunction|DrawSpeed)
  (CallFunction|DrawHealth)
  (CallFunction|CheckDead)
  (bind _returnvalue (Class|PlayerController|IsDead))
  (Variables|Default|SetlastDead _returnvalue))

(fn ConstructionScript)

(fn DrawSpeed
  (bind _returnvalue (Class|PlayerController|IsDead))
  (if (not _returnvalue)
    (bind _returnvalue_2 (Class|PlayerController|GetLocalPlayerID))
    (bind _asplayer_hudnon_umg (Utilities|Casting|CastToPlayerHUDnonUMG (HUD|GetHUD)))
    (Default|SetSpeed _asplayer_hudnon_umg (Utilities|Text|ToText(Float) (Math|Vector2D|Vector2DLength (Math|Conversions|ToVector2D(Vector) (Variables|/Script/Engine.MovementComponent|GetVelocity (Variables|/Script/Engine.Character|GetCharacterMovement (Game|GetPlayerCharacter (Math|Conversions|ToInteger(Byte) _returnvalue_2)))))) "HalfToEven"))))

(fn CheckDead
  (bind _returnvalue (HUD|GetHUD))
  (bind _returnvalue_2 (Class|PlayerController|IsDead))
  (if (Math|Boolean|NotEqual(Boolean) _returnvalue_2 (Variables|Default|GetlastDead))
    (bind _returnvalue_3 (Class|PlayerController|IsDead))
    (if _returnvalue_3
      (bind _asplayer_hudnon_umg (Utilities|Casting|CastToPlayerHUDnonUMG _returnvalue))
      (Default|SetHideCrossHair _asplayer_hudnon_umg true)
      (else
        (bind _asplayer_hudnon_umg_2 (Utilities|Casting|CastToPlayerHUDnonUMG _returnvalue))
        (Default|SetHideCrossHair _asplayer_hudnon_umg_2 false)))))

(fn DrawHealth
  (bind _returnvalue (Class|PlayerController|IsDead))
  (if (not _returnvalue)
    (bind _returnvalue_2 (Class|PlayerController|GetLocalPlayerID))
    (if (not (== (Game|GetPlayerCharacter (Math|Conversions|ToInteger(Byte) _returnvalue_2)) 0))
      (bind _asplayer_character (Utilities|Casting|CastToPlayerCharacter (Game|GetPlayerCharacter (Math|Conversions|ToInteger(Byte) _returnvalue_2))))
      (bind _returnvalue_3 (Class|PlayerCharacter|GetCurHealth _asplayer_character))
      (bind _asplayer_hudnon_umg (Utilities|Casting|CastToPlayerHUDnonUMG (HUD|GetHUD)))
      (Default|SetHealth _asplayer_hudnon_umg (Utilities|Text|ToText(Integer) _returnvalue_3)))))