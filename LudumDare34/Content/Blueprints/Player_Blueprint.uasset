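; Player character Blueprint that routes overlap events from two trigger components, WallHoldTrigger and HitHeadBox, to handler functions defined outside this graph.
; Begin overlaps call EnterWallBox and EnterHeadBox respectively, passing the overlap data through.
; Both end overlaps call ExitWallBox, so the head box has no separate exit handler here.
; The construction script is empty, and a horizontal-speed-to-text node chain is left unused.
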(event OnComponentBeginOverlap(WallHoldTrigger)
  (params (OtherActor :type Actor%20Object%20Reference) (OtherComp :type Primitive%20Component%20Object%20Reference) (OtherBodyIndex :type Integer) (bFromSweep :type Boolean) (SweepResult :type Hit%20Result%20Structure%20%28by%20ref%29))
  (Class|PlayerCharacter|EnterWallBox OtherActor OtherComp OtherBodyIndex bFromSweep SweepResult))

(event OnComponentEndOverlap(WallHoldTrigger)
  (params (OtherActor :type Actor%20Object%20Reference) (OtherComp :type Primitive%20Component%20Object%20Reference) (OtherBodyIndex :type Integer))
  (Class|PlayerCharacter|ExitWallBox OtherActor OtherComp OtherBodyIndex))

(event OnComponentBeginOverlap(HitHeadBox)
  (params (OtherActor :type Actor%20Object%20Reference) (OtherComp :type Primitive%20Component%20Object%20Reference) (OtherBodyIndex :type Integer) (bFromSweep :type Boolean) (SweepResult :type Hit%20Result%20Structure%20%28by%20ref%29))
  (Class|PlayerCharacter|EnterHeadBox OtherActor OtherComp OtherBodyIndex bFromSweep SweepResult))

(event OnComponentEndOverlap(HitHeadBox)
  (params (OtherActor :type Actor%20Object%20Reference) (OtherComp :type Primitive%20Component%20Object%20Reference) (OtherBodyIndex :type Integer))
  (Class|PlayerCharacter|ExitWallBox OtherActor OtherComp OtherBodyIndex))

(fn ConstructionScript)