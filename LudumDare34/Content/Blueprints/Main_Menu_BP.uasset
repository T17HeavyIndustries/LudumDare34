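; Main menu Blueprint that lets the player choose a player count from one to four using clickable hit components and text renders.
; Clicking an option turns its text red, resets the other three to white, and passes the count to Main_Menu_GameMode_BP.
; The Play button only prints a placeholder message, and the construction script prints a leftover debug string.
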(event OnClicked(PlayHit)
  (params (TouchedComponent :type Primitive%20Component%20Object%20Reference))
  (Development|PrintString "Hello"))

(event OnClicked(Players2hit)
  (params (TouchedComponent :type Primitive%20Component%20Object%20Reference))
  (Rendering|Components|TextRender|SetTextRenderColor (Variables|Default|GetPlayers%202) (Math|Color|MakeColor 0 0 255 255))
  (Rendering|Components|TextRender|SetTextRenderColor (Variables|Default|GetPlayers%201) (Math|Color|MakeColor 255 255 255 255))
  (bind _asmain_menu_game_mode_bp (Utilities|Casting|CastToMain_Menu_GameMode_BP (Game|GetGameMode)))
  (Class|MainMenu|SetPlayerCount _asmain_menu_game_mode_bp 2))

(event OnClicked(Players3hit)
  (params (TouchedComponent :type Primitive%20Component%20Object%20Reference))
  (Rendering|Components|TextRender|SetTextRenderColor (Variables|Default|GetPlayers%203) (Math|Color|MakeColor 0 0 255 255))
  (Rendering|Components|TextRender|SetTextRenderColor (Variables|Default|GetPlayers%201) (Math|Color|MakeColor 255 255 255 255))
  (bind _asmain_menu_game_mode_bp (Utilities|Casting|CastToMain_Menu_GameMode_BP (Game|GetGameMode)))
  (Class|MainMenu|SetPlayerCount _asmain_menu_game_mode_bp 3))

(event OnClicked(Players4hit)
  (params (TouchedComponent :type Primitive%20Component%20Object%20Reference))
  (Rendering|Components|TextRender|SetTextRenderColor (Variables|Default|GetPlayers%204) (Math|Color|MakeColor 0 0 255 255))
  (Rendering|Components|TextRender|SetTextRenderColor (Variables|Default|GetPlayers%201) (Math|Color|MakeColor 255 255 255 255))
  (bind _asmain_menu_game_mode_bp (Utilities|Casting|CastToMain_Menu_GameMode_BP (Game|GetGameMode)))
  (Class|MainMenu|SetPlayerCount _asmain_menu_game_mode_bp 4))

(event OnClicked(Players1hit)
  (params (TouchedComponent :type Primitive%20Component%20Object%20Reference))
  (Rendering|Components|TextRender|SetTextRenderColor (Variables|Default|GetPlayers%201) (Math|Color|MakeColor 0 0 255 255))
  (Rendering|Components|TextRender|SetTextRenderColor (Variables|Default|GetPlayers%202) (Math|Color|MakeColor 255 255 255 255))
  (bind _asmain_menu_game_mode_bp (Utilities|Casting|CastToMain_Menu_GameMode_BP (Game|GetGameMode)))
  (Class|MainMenu|SetPlayerCount _asmain_menu_game_mode_bp 1))

(fn ConstructionScript
  (Development|PrintString "penis"))