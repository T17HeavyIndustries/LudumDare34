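; Laser gun Blueprint that draws a beam particle effect when its FireLaser event runs with the trigger held.
; Each call deactivates the previous emitter, then spawns and stores a new one only if TriggerHeld is true.
; The beam starts at the actor's location, and FindEndLocation computes its end from PlayerArrow's world position and forward vector.
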(event EventFireLaser
  (bind _returnvalue (Transformation|GetActorLocation))
  (bind _playerarrow (Variables|Default|GetplayerArrow))
  (Components|Activation|Deactivate (Variables|Default|GettempEmitter))
  (if (Variables|Default|GettriggerHeld)
    (bind _returnvalue_2 (Effects|SpawnEmitteratLocation "/Game/Textures/lasel_particle.lasel_particle" _returnvalue))
    (Variables|Default|SettempEmitter _returnvalue_2)
    (Class|ParticleSystemComponent|SetBeamSourcePoint _returnvalue_2 0 _returnvalue)
    (bind _returnvalue_3 (Class|Gun|FindEndLocation (Transformation|GetWorldLocation _playerarrow) (Math|Vector|GetForwardVector _playerarrow)))
    (Class|ParticleSystemComponent|SetBeamEndPoint _returnvalue_2 0 _returnvalue_3)))

(fn ConstructionScript)